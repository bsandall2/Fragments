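; Collectable pickup actor that the player collects with the Interact input while inside its Box trigger.
; Overlap by BP_Player enables input on the actor and shows an interact prompt widget; leaving disables input and notifies that prompt.
; Interacting decrements CollectablesLeft on GameModeBP, adds a collectables widget to the viewport, plays a pickup sound and destroys the actor.
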(event `InputAction|Interact`
  (params (Key :type "Key Structure"))
  (:`Pressed`
    (bind _asgame_mode_bp (cast `/Game/GameModeBP` (`GameplayStatics.GetGameMode`)))
    (bind _result (`/Engine/EditorBlueprintResources/StandardMacros.DecrementInt` (`/Game/GameModeBP.Collectables left` _asgame_mode_bp))
      (:`  `
        (set `/Game/GameModeBP.Collectables left` _result _asgame_mode_bp)
        (bind _returnvalue (`|CreateWidget` "/Game/InteractItems/CollectablesWidget.CollectablesWidget_C"))
        (`UserWidget.AddToViewport` _returnvalue 0)
        (`GameplayStatics.PlaySound2D` "/Game/Sounds/SFX/PickUpSFX.PickUpSFX" 1.0 1.0 0.0 null null)
        (`self.K2_DestroyActor`)))))

(event `self.Box.OnComponentBeginOverlap`
  (params (OverlappedComponent :type "PrimitiveComponent Object Reference") (OtherActor :type "Actor Object Reference") (OtherComp :type "PrimitiveComponent Object Reference") (OtherBodyIndex :type Integer) (bFromSweep :type Boolean) (SweepResult :type "HitResult Structure (by ref)"))
  (cast `/Game/Player/BP_Player` OtherActor)
  (`self.EnableInput` (`GameplayStatics.GetPlayerController` 0))
  (bind _returnvalue (`|CreateWidget` "/Game/InteractItems/InteractPromptWidget.InteractPromptWidget_C"))
  (`UserWidget.AddToViewport` _returnvalue 0))

(event `self.Box.OnComponentEndOverlap`
  (params (OverlappedComponent :type "PrimitiveComponent Object Reference") (OtherActor :type "Actor Object Reference") (OtherComp :type "PrimitiveComponent Object Reference") (OtherBodyIndex :type Integer))
  (cast `/Game/Player/BP_Player` OtherActor)
  (`self.DisableInput` (`GameplayStatics.GetPlayerController` 0))
  (`/Game/InteractItems/InteractPromptWidget.PlayerLeavesInteract` (stale `self.Box.OnComponentBeginOverlap` _returnvalue)))

(fn `UserConstructionScript`)