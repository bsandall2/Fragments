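; BP_Player is the player Blueprint, handling walking, looking, and movement feedback through camera shake and footstep audio.
; Axis inputs drive movement relative to control yaw and add clamped pitch and yaw look input.
; Both movement axes share a horizontal velocity check feeding two mutually resetting DoOnce gates.
; These gates start the shake and footsteps once when motion begins, then stop them when it ends.
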(event `InputAxis|Move Forwards/Backwards`
  (params (AxisValue :type "Float (single-precision)"))
  (bind (_returnvalue_x _returnvalue_y) (`KismetMathLibrary.BreakVector` (`self.GetVelocity`)))
  (bind _footsteps (`self.Footsteps`))
  ;[1 1 1] Movement
  (`self.AddMovementInput` (`KismetMathLibrary.GetForwardVector` (`KismetMathLibrary.MakeRotator` 0.0 0.0 (.yaw (`self.GetControlRotation`)))) AxisValue)
  ;[1 1 1] Camera Shake on movement
  (if (or (> _returnvalue_x 1.0) (< _returnvalue_x -1.0) (> _returnvalue_y 1.0) (< _returnvalue_y -1.0)) :!label _label
    (`/Engine/EditorBlueprintResources/StandardMacros.DoOnce` false :!label _label_2
      (:`Completed`
        (`self.Start Camera Shake`)
        (`AudioComponent.Play` _footsteps 0.0)
        (goto _label_3 :!via `Reset`)))
    (else
      (`/Engine/EditorBlueprintResources/StandardMacros.DoOnce` false :!label _label_3
        (:`Completed`
          (`self.Stop Camera Shake`)
          (`AudioComponent.Stop` _footsteps)
          (goto _label_2 :!via `Reset`))))))

(event `InputAxis|Move Left/Right`
  (params (AxisValue :type "Float (single-precision)"))
  ;[1 1 1] Movement
  (`self.AddMovementInput` (`KismetMathLibrary.GetRightVector` (`KismetMathLibrary.MakeRotator` 0.0 0.0 (.yaw (`self.GetControlRotation`)))) AxisValue)
  (goto _label))

(event `InputAxis|Look up/down`
  (params (AxisValue :type "Float (single-precision)"))
  ;[1 1 1] Look around
  (`self.AddControllerPitchInput` (`KismetMathLibrary.FClamp` AxisValue -1.0)))

(event `Start Camera Shake`
  ;[1 1 1] Stop and Start camera shake
  (bind _returnvalue (`PlayerCameraManager.StartCameraShake` :`self` (`GameplayStatics.GetPlayerCameraManager` 0) :`ShakeClass` "/Game/Player/CameraShakeMovement.CameraShakeMovement_C")))

(event `InputAxis|Look left/Right`
  (params (AxisValue :type "Float (single-precision)"))
  ;[1 1 1] Look around
  (`self.AddControllerYawInput` (`KismetMathLibrary.FClamp` AxisValue -1.0)))

(event `Stop Camera Shake`
  ;[1 1 1] Stop and Start camera shake
  (`PlayerCameraManager.StopCameraShake` (`GameplayStatics.GetPlayerCameraManager` 0) (stale `Start Camera Shake` _returnvalue) false))

(fn `UserConstructionScript`)