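; First-person player Blueprint with movement, look, a walking camera shake and pick-up-to-inspect for items tagged "Interactable".
; DoOnce gates start and stop the shake as horizontal velocity changes.
; Interact line-traces from the camera, copies the hit's class into the ItemActor child actor, destroys the original and lerps it to Arrow1 before calling StartInspect.
; Interacting again reverses the timeline, spawns a fresh copy and lowers it onto the surface below.
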(event `InputAxis|Move Forwards/Backwards`
  (params (AxisValue :type "Float (single-precision)"))
  (bind (_returnvalue_x _returnvalue_y) (`KismetMathLibrary.BreakVector` (`self.GetVelocity`)))
  ;[1 1 1] Movement
  (`self.AddMovementInput` (`KismetMathLibrary.GetForwardVector` (`KismetMathLibrary.MakeRotator` 0.0 0.0 (.yaw (`self.GetControlRotation`)))) AxisValue)
  ;[1 1 1] Camera Shake on movement
  (if (or (> _returnvalue_x 1.0) (< _returnvalue_x -1.0) (> _returnvalue_y 1.0) (< _returnvalue_y -1.0)) :!label _label
    (`/Engine/EditorBlueprintResources/StandardMacros.DoOnce` false :!label _label_2
      (:`Completed`
        (`self.Start Camera Shake`)
        (goto _label_3 :!via `Reset`)))
    (else
      (`/Engine/EditorBlueprintResources/StandardMacros.DoOnce` false :!label _label_3
        (:`Completed`
          (`self.Stop Camera Shake`)
          (goto _label_2 :!via `Reset`))))))

(event `InputAxis|Move Left/Right`
  (params (AxisValue :type "Float (single-precision)"))
  ;[1 1 1] Movement
  (`self.AddMovementInput` (`KismetMathLibrary.GetRightVector` (`KismetMathLibrary.MakeRotator` 0.0 0.0 (.yaw (`self.GetControlRotation`)))) AxisValue)
  (goto _label))

(event `InputAxis|Look up/down`
  (params (AxisValue :type "Float (single-precision)"))
  ;[1 1 1] Look around
  (`self.AddControllerPitchInput` (`KismetMathLibrary.FClamp` AxisValue -1.0)))

(event `Start Camera Shake`
  ;[1 1 1] Stop and Start camera shake
  (bind _returnvalue (`PlayerCameraManager.StartCameraShake` :`self` (`GameplayStatics.GetPlayerCameraManager` 0) :`ShakeClass` "/Game/CameraShakeMovement.CameraShakeMovement_C")))

(event `Inspect`
  (bind _camera (`self.Camera`))
  (bind _itemactor (`self.ItemActor`))
  (bind _returnvalue (`SceneComponent.K2_GetComponentLocation` _camera))
  (bind _returnvalue_2 (`self.K2_GetActorLocation` (`self.PlacedItem`)))
  ;[1 1 1] Item pick up and put down
  (bind (_outhit _returnvalue_3) (`KismetSystemLibrary.LineTraceSingle` _returnvalue (+ _returnvalue (* (`SceneComponent.GetForwardVector` _camera) 150.0)) "TraceTypeQuery1" :!label _label_4))
  (if _returnvalue_3
    (bind (_bblockinghit _binitialoverlap _time _distance _location _impactpoint _normal _impactnormal _physmat _hitactor) (`GameplayStatics.BreakHitResult` _outhit))
    (if (`self.ActorHasTag` _hitactor "Interactable")
      (`|ExecutionSequence`
        (:`then_0`
          (`KismetSystemLibrary.Delay` 0.1)
          (if (not (`self.Inspecting?`))
            (set `self.Inspecting?` true)
            (set `self.StartLoc` (`SceneComponent.RelativeLocation` (`self.ItemActor`)))
            (set `self.EndLoc` (`SceneComponent.RelativeLocation` (`self.Arrow1`)))
            (bind (_direction _itemtrack) (`Timeline|PickUpItem` :!label _label_5)
              (:`Update`
                (`SceneComponent.K2_SetRelativeLocation` (`self.ItemActor`) (`KismetMathLibrary.VLerp` (`self.StartLoc`) (`self.EndLoc`) _itemtrack) false false))
              (:`Finished`
                (if (`self.Inspecting?`)
                  (bind _asinspect_item_parent (cast `/Game/InteractItems/InspectItemParent` (`ChildActorComponent.ChildActor` (`self.ItemActor`))))
                  (`/Game/InteractItems/InspectItemParent.Start inspect` _asinspect_item_parent self)
                  (else
                    (bind _returnvalue_4 (`|SpawnActorFromClass` (`ChildActorComponent.ChildActorClass` (`self.ItemActor`)) (`KismetMathLibrary.MakeTransform` (`KismetMathLibrary.TransformLocation` (`SceneComponent.K2_GetComponentToWorld` (`self.Camera`)) (`SceneComponent.RelativeLocation` (`self.ItemActor`)))) "Undefined" "OverrideRootScale" null null))
                    (set `self.PlacedItem` _returnvalue_4)
                    (`ChildActorComponent.SetChildActorClass` (`self.ItemActor`) null)
                    (`self.ResetDoOnce`)
                    (bind _outhit_2 (`KismetSystemLibrary.LineTraceSingle` _returnvalue_2 (- _returnvalue_2 (0.0 0.0 1000.0)) "TraceTypeQuery1" false (`|MakeArray` (`self.PlacedItem`))))
                    (set `self.NewEndLoc` (`.Location` (`GameplayStatics.BreakHitResult` _outhit_2)))
                    (set `self.NewStartLoc` (`self.K2_GetActorLocation` (`self.PlacedItem`)))
                    (bind (_direction_2 _fixloctrack) (`Timeline|FixLoc` :!via `PlayFromStart`)
                      (:`Update`
                        (`self.K2_SetActorLocation` (`self.PlacedItem`) (`KismetMathLibrary.VLerp` (`self.NewStartLoc`) (`self.NewEndLoc`) _fixloctrack) false false)))))))
            (else
              (set `self.Inspecting?` false)
              (goto _label_5 :!via `Reverse`))))
        (:`then_1`
          (`/Engine/EditorBlueprintResources/StandardMacros.DoOnce` false :!label _label_6
            (:`Completed`
              (`ChildActorComponent.SetChildActorClass` _itemactor (`GameplayStatics.GetObjectClass` _hitactor))
              (`SceneComponent.K2_SetRelativeLocation` _itemactor (`KismetMathLibrary.InverseTransformLocation` (`SceneComponent.K2_GetComponentToWorld` (`self.Camera`)) (`self.K2_GetActorLocation` _hitactor)) false false)
              (`self.K2_DestroyActor` _hitactor))))))))

(event `InputAxis|Look left/Right`
  (params (AxisValue :type "Float (single-precision)"))
  ;[1 1 1] Look around
  (`self.AddControllerYawInput` (`KismetMathLibrary.FClamp` AxisValue -1.0)))

(event `InputAction|Interact`
  (params (Key :type "Key Structure"))
  ;[1 1 1] Item pick up and put down
  (:`Pressed`
    (goto _label_4)))

(event `Stop Camera Shake`
  ;[1 1 1] Stop and Start camera shake
  (`PlayerCameraManager.StopCameraShake` (`GameplayStatics.GetPlayerCameraManager` 0) (stale `Start Camera Shake` _returnvalue) false))

(event `ResetDoOnce`
  ;[1 1 1] Item pick up and put down
  (goto _label_6 :!via `Reset`))

(fn `UserConstructionScript`)